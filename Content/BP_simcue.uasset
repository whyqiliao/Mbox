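; Test Blueprint that drives a six-DOF motion platform and its physical effects through the lcsimcue object.
; BeginPlay initialises the platform, moves it to middle, waits out the move, then opens a gate; EndPlay closes the UDP port.
; NumPad 2 passes through that gate to send random angles and accelerations to the inverse solution.
; NumPad 1 alternates FX writes for smoke, wind, rain, lightning and fire, starting with off.
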(event `Key|NumPadOne`
  (params (Key :type "Key Structure"))
  (bind _returnvalue (`lcsimcueobject.getlcsimcueobjectObject`))
  (:`Pressed`
    (`/Engine/EditorBlueprintResources/StandardMacros.FlipFlop`
      (:`A`
        (`lcsimcueobject.WriteFXControl` _returnvalue (make `MboxFXStruct` false false false false false)))
      (:`B`
        (`lcsimcueobject.WriteFXControl` _returnvalue (make `MboxFXStruct` true true true true true true))))))

(event `self.ReceiveBeginPlay`
  (bind _returnvalue (`lcsimcueobject.getlcsimcueobjectObject`))
  (bind _returnvalue_2 (`KismetMathLibrary.RandomFloatInRange` 0.0 10.0))
  (bind _returnvalue_3 (`KismetMathLibrary.RandomFloatInRange` 0.0 5.0))
  (`lcsimcueobject.Choose_PlatformTypeAndInit` :`self` _returnvalue :`PlatformType` 1)
  (`KismetSystemLibrary.Delay` 0.2)
  (`lcsimcueobject.GoMiddlePlatform` _returnvalue 3000)
  (`KismetSystemLibrary.Delay` (* 3000 0.001))
  (goto _label :!via `Open`))

(event `Key|NumPadTwo`
  (params (Key :type "Key Structure"))
  (bind _returnvalue (`KismetMathLibrary.RandomFloatInRange` 0.0 10.0))
  (bind _returnvalue_2 (`KismetMathLibrary.RandomFloatInRange` 0.0 5.0))
  (:`Pressed`
    (`/Engine/EditorBlueprintResources/StandardMacros.Gate` true :!label _label
      (:`Exit`
        (`lcsimcueobject.Cue2Inverse_Solution` (`lcsimcueobject.getlcsimcueobjectObject`) (make `UE_DOF6_GAME_PARA` _returnvalue_2 _returnvalue_2 _returnvalue_2 _returnvalue _returnvalue _returnvalue))))))

(event `self.ReceiveEndPlay`
  (params (EndPlayReason :type "EEndPlayReason Enum" :default "Destroyed"))
  (`lcsimcueobject.CloseMboxUdpPort` (`lcsimcueobject.getlcsimcueobjectObject`)))

(fn `UserConstructionScript`)