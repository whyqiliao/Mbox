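; BPC_simcue, a Blueprint component that drives a 6DOF motion simulator platform and its effects hardware through a simcue object.
; BeginPlay initializes the chosen platform type, moves it to middle position, then opens a gate once that move time elapses.
; Only then do Cue_2Inverse_Solution calls pass motion parameters to the inverse solution.
; UpdateCueFX writes a bitmask for six effect switches, and EndPlay closes the UDP port.
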(event `self.ReceiveBeginPlay`
  (bind _returnvalue (`lcsimcueobject.getlcsimcueobjectObject`))
  (bind _returnvalue_2 (`KismetSystemLibrary.MakeLiteralInt` (`self.GoMiddleTime_ms`)))
  (`lcsimcueobject.Choose_PlatformTypeAndInit` _returnvalue (`self.PlatformType`) (`self.Dof6SysPara`))
  (`KismetSystemLibrary.Delay` 0.2)
  (`lcsimcueobject.GoMiddlePlatform` _returnvalue _returnvalue_2)
  (`KismetSystemLibrary.Delay` (* _returnvalue_2 0.001))
  (goto _label :!via `Open`))

(event `Cue_2Inverse_Solution`
  (params (dof6_game_para :type "UE_DOF6_GAME_PARA Structure"))
  (`/Engine/EditorBlueprintResources/StandardMacros.Gate` true :!label _label
    (:`Exit`
      (`lcsimcueobject.Cue2Inverse_Solution` (`lcsimcueobject.getlcsimcueobjectObject`) dof6_game_para))))

(event `UpdateCueFX`
  (params (newFXState :type Byte))
  (`lcsimcueobject.WriteFXControl` (`lcsimcueobject.getlcsimcueobjectObject`) (`KismetMathLibrary.Conv_ByteToInt` newFXState)))

(event `self.ReceiveEndPlay`
  (params (EndPlayReason :type "EEndPlayReason Enum" :default "Destroyed"))
  (`lcsimcueobject.CloseMboxUdpPort` (`lcsimcueobject.getlcsimcueobjectObject`)))